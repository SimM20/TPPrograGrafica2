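; Actor base with an editable material, exposing a change event for a named parameter value.
; The construction script creates a dynamic instance of slot 0's material on the skeletal mesh if it has a valid asset, otherwise on the static mesh.
; It stores that instance in DynamicMaterial and applies it to the mesh.
; ChangeMaterialValue forwards the value and parameter name to OnValueChanged, which is empty here.
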(event Custom|ChangeMaterialValue
  (params (NewValue :type Float%20%28double-precision%29) (ParamName :type Name))
  (CallFunction|OnValueChanged NewValue ParamName))

(fn ConstructionScript
  (Utilities|IsValid (Variables|/Script/Engine.SkeletalMeshComponent|GetSkeletalMeshAsset (Variables|Default|GetSkeletalMesh))
    (:Is%20Valid
      (bind _returnvalue (Rendering|Material|CreateDynamicMaterialInstance (Rendering|Material|GetMaterial (Variables|Default|GetSkeletalMesh) 0) "None" "None" :!class /Script/Engine.KismetMaterialLibrary))
      (bind _output_get (Variables|Default|SetDynamicMaterial _returnvalue))
      (Rendering|Material|SetMaterial (Variables|Default|GetSkeletalMesh) 0 _output_get))
    (:Is%20Not%20Valid
      (bind _returnvalue_2 (Rendering|Material|CreateDynamicMaterialInstance (Rendering|Material|GetMaterial (Variables|Default|GetStaticMesh) 0) "None" "None" :!class /Script/Engine.KismetMaterialLibrary))
      (bind _output_get_2 (Variables|Default|SetDynamicMaterial _returnvalue_2))
      (Rendering|Material|SetMaterial (Variables|Default|GetStaticMesh) 0 _output_get_2))))

(fn OnValueChanged
  (params (NewValue :type Float%20%28double-precision%29) (ParamName :type Name)))